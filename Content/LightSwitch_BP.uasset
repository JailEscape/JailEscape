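; Interactable light switch that the player toggles on and off when nearby.
; Overlapping the interact zone enables input for the first-person character; leaving disables it unless a dialog is open.
; Interact with the cursor over the click zone plays a sound, flips IsOn and raises Activator, which Tick clears as a momentary signal.
; Tick also rotates the switch mesh toward its on or off roll at constant speed.
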(event `self.InteractZone.OnComponentBeginOverlap`
  (params (OverlappedComponent :type "PrimitiveComponent Object Reference") (OtherActor :type "Actor Object Reference") (OtherComp :type "PrimitiveComponent Object Reference") (OtherBodyIndex :type Integer) (bFromSweep :type Boolean) (SweepResult :type "HitResult Structure (by ref)"))
  (cast `/Game/FirstPersonCPP/Blueprints/FirstPersonCharacter` OtherActor)
  (`self.EnableInput` (`GameplayStatics.GetPlayerController` 0)))

(event `self.ReceiveTick`
  (params (DeltaSeconds :type "Float (single-precision)"))
  (bind _lightswitch (`self.LightSwitch`))
  (bind (_relativerotation_roll _relativerotation_pitch _relativerotation_yaw) (`KismetMathLibrary.BreakRotator` (`SceneComponent.RelativeRotation` _lightswitch)))
  (`|ExecutionSequence`
    (:`then_0`
      (set `self.activator` false))
    (:`then_1`
      (`SceneComponent.K2_SetRelativeRotation` _lightswitch (`KismetMathLibrary.RInterpTo_Constant` (`SceneComponent.RelativeRotation` _lightswitch) (`KismetMathLibrary.MakeRotator` (`self.switchRot`) _relativerotation_pitch _relativerotation_yaw) (`GameplayStatics.GetWorldDeltaSeconds`) 130.0) false false))))

(event `self.InteractZone.OnComponentEndOverlap`
  (params (OverlappedComponent :type "PrimitiveComponent Object Reference") (OtherActor :type "Actor Object Reference") (OtherComp :type "PrimitiveComponent Object Reference") (OtherBodyIndex :type Integer))
  (bind _asfirst_person_character (cast `/Game/FirstPersonCPP/Blueprints/FirstPersonCharacter` OtherActor))
  (if (not (`MyProjectCharacter.isDialogOpen` _asfirst_person_character))
    (`self.DisableInput` (`GameplayStatics.GetPlayerController` 0))))

(event `InputAction|Interact`
  (params (Key :type "Key Structure" :default "AnyKey"))
  (:`Pressed`
    (if (== (`.HitComponent` (`GameplayStatics.BreakHitResult` (`PlayerController.GetHitResultUnderCursorByChannel` (`GameplayStatics.GetPlayerController` 0) "TraceTypeQuery1" false))) (`self.ClickZone`))
      (`|ExecutionSequence`
        (:`then_0`
          (`AudioComponent.Play` (`self.ClickSound`) 0.0))
        (:`then_1`
          (if (`self.isOn`)
            (set `self.isOn` false)
            (set `self.switchRot` 0.0)
            (else
              (set `self.isOn` true)
              (set `self.switchRot` 70.0))))
        (:`then_3`
          (set `self.activator` true))))))

(fn `UserConstructionScript`)