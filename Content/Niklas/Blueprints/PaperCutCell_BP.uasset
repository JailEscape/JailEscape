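; Pickup actor for a paper cut cell that shows one of ten cell meshes, chosen at random on BeginPlay.
; The InteractionZone enables input when the FirstPersonCharacter enters and disables it on exit unless a dialog is open.
; Pressing Interact with the cursor over InteractionObject plays a sound, hides the chosen mesh and sets IsPickedUp to block repeat pickups.
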(event `self.ReceiveBeginPlay`
  (bind _returnvalue (`KismetMathLibrary.RandomIntegerInRange` 0 9))
  (`|ExecutionSequence`
    (:`then_0`
      (bind _output_get (set `self.nPaperIndex` _returnvalue))
      (bind _meshtoactivate (`self.GetMeshByIndex` _output_get))
      (`SceneComponent.SetVisibility` _meshtoactivate true false))
    (:`then_1`
      (`KismetSystemLibrary.PrintString` (`KismetStringLibrary.Conv_IntToString` _returnvalue) true true (struct :`R` 0.175231 :`G` 1.0 :`A` 1.0)))))

(event `self.interactionZone.OnComponentBeginOverlap`
  (params (OverlappedComponent :type "PrimitiveComponent Object Reference") (OtherActor :type "Actor Object Reference") (OtherComp :type "PrimitiveComponent Object Reference") (OtherBodyIndex :type Integer) (bFromSweep :type Boolean) (SweepResult :type "HitResult Structure (by ref)"))
  (cast `/Game/FirstPersonCPP/Blueprints/FirstPersonCharacter` OtherActor)
  (`self.EnableInput` (`GameplayStatics.GetPlayerController` 0))
  (`KismetSystemLibrary.PrintString` "Input Enabled" true false (struct :`G` 0.66 :`B` 1.0 :`A` 1.0) 4.0))

(event `self.interactionZone.OnComponentEndOverlap`
  (params (OverlappedComponent :type "PrimitiveComponent Object Reference") (OtherActor :type "Actor Object Reference") (OtherComp :type "PrimitiveComponent Object Reference") (OtherBodyIndex :type Integer))
  (bind _asfirst_person_character (cast `/Game/FirstPersonCPP/Blueprints/FirstPersonCharacter` OtherActor))
  (if (not (`MyProjectCharacter.isDialogOpen` _asfirst_person_character))
    (`self.DisableInput` (`GameplayStatics.GetPlayerController` 0))
    (`KismetSystemLibrary.PrintString` "Input Disabled" true false (struct :`G` 0.66 :`B` 1.0 :`A` 1.0) 4.0)))

(event `InputAction|Interact`
  (params (Key :type "Key Structure" :default "AnyKey"))
  (:`Pressed`
    (if (and (== (`.HitComponent` (`GameplayStatics.BreakHitResult` (`PlayerController.GetHitResultUnderCursorByChannel` (`GameplayStatics.GetPlayerController` 0) "TraceTypeQuery1" false))) (`self.interactionObject`)) (not (`self.bIsPickedUp`)))
      (`|ExecutionSequence`
        (:`then_0`
          (`AudioComponent.Play` (`self.pickupSound`) 0.0))
        (:`then_1`
          (bind _meshtoactivate (`self.GetMeshByIndex` (`self.nPaperIndex`))))
        (:`then_2`
          (`SceneComponent.SetVisibility` _meshtoactivate false false))
        (:`then_3`
          (set `self.bIsPickedUp` true))
        (:`then_4`
          (`KismetSystemLibrary.PrintString` "Clicked on PaperCutCellBlock" true true (struct :`R` 1.0 :`G` 0.24256 :`A` 1.0)))))))

(fn `GetMeshByIndex`
  (params (MeshIndex :type Integer))
  (returns (MeshToActivate :type "StaticMeshComponent Object Reference"))
  (`|ExecutionSequence`
    (:`then_0`
      (if (== MeshIndex 0)
        (return (`self.cell1`))))
    (:`then_1`
      (if (== MeshIndex 1)
        (return (`self.cell2`))))
    (:`then_2`
      (if (== MeshIndex 2)
        (return (`self.cell3`))))
    (:`then_3`
      (if (== MeshIndex 3)
        (return (`self.cell4`))))
    (:`then_4`
      (if (== MeshIndex 4)
        (return (`self.cell5`))))
    (:`then_5`
      (if (== MeshIndex 5)
        (return (`self.cell6`))))
    (:`then_6`
      (if (== MeshIndex 6)
        (return (`self.cell7`))))
    (:`then_7`
      (if (== MeshIndex 7)
        (return (`self.cell8`))))
    (:`then_8`
      (if (== MeshIndex 8)
        (return (`self.cell9`))))
    (:`then_9`
      (if (== MeshIndex 9)
        (return (`self.cell10`))))))

(fn `UserConstructionScript`)