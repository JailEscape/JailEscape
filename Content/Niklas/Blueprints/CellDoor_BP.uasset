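; Sliding cell door that the player opens and closes by interacting with it while inside its interaction zone, unless it is locked.
; Overlap enables input for the actor, and leaving disables it unless the character has a dialog open.
; Interact checks the cursor trace hits the door, then flips the target position and plays a sound.
; Tick interpolates the door along local X and derives open and moving states from position thresholds, blocking toggles mid-slide.
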(event `self.interactionZone.OnComponentBeginOverlap`
  (params (OverlappedComponent :type "PrimitiveComponent Object Reference") (OtherActor :type "Actor Object Reference") (OtherComp :type "PrimitiveComponent Object Reference") (OtherBodyIndex :type Integer) (bFromSweep :type Boolean) (SweepResult :type "HitResult Structure (by ref)"))
  (cast `/Game/FirstPersonCPP/Blueprints/FirstPersonCharacter` OtherActor)
  (`self.EnableInput` (`GameplayStatics.GetPlayerController` 0))
  (`KismetSystemLibrary.PrintString` "Input Enabled" true false (struct :`G` 0.66 :`B` 1.0 :`A` 1.0) 4.0))

(event `self.ReceiveTick`
  (params (DeltaSeconds :type "Float (single-precision)"))
  (bind _door (`self.door`))
  (bind _relativelocation (`SceneComponent.RelativeLocation` _door))
  (bind (_relativelocation_x _relativelocation_y _relativelocation_z) (`KismetMathLibrary.BreakVector` (`SceneComponent.RelativeLocation` _door)))
  (if (not (`self.isLocked_0`))
    (`|ExecutionSequence`
      (:`then_0`
        (bind (_nearopenedpos _nearclosedpos) (`self.CheckForDoorBoundries` _relativelocation))
        (`|ExecutionSequence`
          (:`then_0`
            (if _nearopenedpos
              (set `self.doorIsOpen` true)))
          (:`then_1`
            (if _nearclosedpos
              (set `self.doorIsOpen` false)))))
      (:`then_1`
        (`SceneComponent.K2_SetRelativeLocation` _door (`KismetMathLibrary.VInterpTo_Constant` _relativelocation (`KismetMathLibrary.MakeVector` (`self.doorPos`) _relativelocation_y _relativelocation_z) (`GameplayStatics.GetWorldDeltaSeconds`) 15.0) false false))
      (:`then_2`
        (set `self.doorIsMoving` (`KismetMathLibrary.BooleanNOR` _nearopenedpos _nearclosedpos))))))

(event `self.interactionZone.OnComponentEndOverlap`
  (params (OverlappedComponent :type "PrimitiveComponent Object Reference") (OtherActor :type "Actor Object Reference") (OtherComp :type "PrimitiveComponent Object Reference") (OtherBodyIndex :type Integer))
  (bind _asfirst_person_character (cast `/Game/FirstPersonCPP/Blueprints/FirstPersonCharacter` OtherActor))
  (if (not (`MyProjectCharacter.isDialogOpen` _asfirst_person_character))
    (`self.DisableInput` (`GameplayStatics.GetPlayerController` 0))
    (`KismetSystemLibrary.PrintString` "Input Disabled" true false (struct :`G` 0.66 :`B` 1.0 :`A` 1.0) 4.0)))

(event `InputAction|Interact`
  (params (Key :type "Key Structure" :default "AnyKey"))
  (bind _doorisopen (`self.doorIsOpen`))
  (bind _returnvalue (not (`self.doorIsMoving`)))
  (:`Pressed`
    (if (not (`self.isLocked_0`))
      (if (== (`.HitComponent` (`GameplayStatics.BreakHitResult` (`PlayerController.GetHitResultUnderCursorByChannel` (`GameplayStatics.GetPlayerController` 0) "TraceTypeQuery1" false))) (`self.door`))
        (`|ExecutionSequence`
          (:`then_0`
            (`KismetSystemLibrary.PrintString` "Clicked On CellDoor" true false (struct :`R` 1.0 :`G` 0.453018 :`A` 1.0))
            (`|ExecutionSequence`
              (:`then_0`
                (if (and _returnvalue (not _doorisopen))
                  (bind _output_get (set `self.doorPos` 0.0))
                  (`KismetSystemLibrary.PrintString` (`KismetStringLibrary.Conv_DoubleToString` _output_get))
                  (`AudioComponent.Play` (`self.doorSound`) 0.0 :!label _label)))
              (:`then_1`
                (if (and _returnvalue _doorisopen)
                  (bind _output_get_2 (set `self.doorPos` -100.0))
                  (`KismetSystemLibrary.PrintString` (`KismetStringLibrary.Conv_DoubleToString` _output_get_2))
                  (goto _label))))))))))

(fn `CheckForDoorBoundries`
  (params (Position :type "Vector Structure"))
  (returns (NearOpenedPos :type Boolean) (NearClosedPos :type Boolean))
  (bind _x (.x Position))
  (`|ExecutionSequence`
    (:`then_2`
      (return (> _x -0.2) (< _x -98.0)))))

(fn `UserConstructionScript`)