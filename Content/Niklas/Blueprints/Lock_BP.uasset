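; Three-wheel combination lock that the first-person player operates with Interact while inside its interaction zone; leaving keeps input enabled if a dialog is open.
; While locked, a cursor trace picks the wheel, advances its wrapping digit index, plays a spin sound and prints the combination.
; Tick eases each wheel toward its digit's angle.
; No combination check lives here, only helpers to play the unlock sound and hide the lock.
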(event `self.interactionZone.OnComponentBeginOverlap`
  (params (OverlappedComponent :type "PrimitiveComponent Object Reference") (OtherActor :type "Actor Object Reference") (OtherComp :type "PrimitiveComponent Object Reference") (OtherBodyIndex :type Integer) (bFromSweep :type Boolean) (SweepResult :type "HitResult Structure (by ref)"))
  (cast `/Game/FirstPersonCPP/Blueprints/FirstPersonCharacter` OtherActor)
  (`self.EnableInput` (`GameplayStatics.GetPlayerController` 0)))

(event `self.interactionZone.OnComponentEndOverlap`
  (params (OverlappedComponent :type "PrimitiveComponent Object Reference") (OtherActor :type "Actor Object Reference") (OtherComp :type "PrimitiveComponent Object Reference") (OtherBodyIndex :type Integer))
  (bind _asfirst_person_character (cast `/Game/FirstPersonCPP/Blueprints/FirstPersonCharacter` OtherActor))
  (if (not (`MyProjectCharacter.isDialogOpen` _asfirst_person_character))
    (`self.DisableInput` (`GameplayStatics.GetPlayerController` 0))))

(event `self.ReceiveTick`
  (params (DeltaSeconds :type "Float (single-precision)"))
  (`|ExecutionSequence`
    (:`then_0`
      (`self.SetMeshRotation` (`self.firstNumWheel`) (stale `InputAction|Interact` _output_get) 36.0 5.0))
    (:`then_1`
      (`self.SetMeshRotation` (`self.secondNumWheel`) (stale `InputAction|Interact` _output_get) 36.0 5.0))
    (:`then_2`
      (`self.SetMeshRotation` (`self.thirdNumWheel`) (stale `InputAction|Interact` _output_get) 36.0 5.0))))

(event `InputAction|Interact`
  (params (Key :type "Key Structure" :default "AnyKey"))
  (:`Pressed`
    (if (and (== (`.HitComponent` (`GameplayStatics.BreakHitResult` (`PlayerController.GetHitResultUnderCursorByChannel` (`GameplayStatics.GetPlayerController` 0) "TraceTypeQuery1" false))) (`self.firstNumWheel`)) (`self.isLocked_0`))
      (`|ExecutionSequence`
        (:`then_1`
          (bind _return_value (`self.CheckForBoundry` (`self.firstWheelIndex`) 10))
          (bind _output_get (set `self.firstWheelIndex` _return_value)))
        (:`then_2`
          (`AudioComponent.Play` (`self.spinSound`) 0.0 :!label _label))
        (:`then_3`
          (`KismetSystemLibrary.PrintString` (`KismetStringLibrary.Concat_StrStr` "Combination Lock: " (`KismetStringLibrary.Conv_IntToString` (`self.firstWheelIndex`)) (`KismetStringLibrary.Conv_IntToString` (`self.secondWheelIndex`)) (`KismetStringLibrary.Conv_IntToString` (`self.thirdWheelIndex`))) true false (struct :`R` 0.525 :`G` 0.525 :`B` 0.525 :`A` 1.0) 1.0 :!label _label_2))))))

(event `InputAction|Interact`
  (params (Key :type "Key Structure" :default "AnyKey"))
  (:`Pressed`
    (if (and (== (`.HitComponent` (`GameplayStatics.BreakHitResult` (`PlayerController.GetHitResultUnderCursorByChannel` (`GameplayStatics.GetPlayerController` 0) "TraceTypeQuery1" false))) (`self.secondNumWheel`)) (`self.isLocked_0`))
      (`|ExecutionSequence`
        (:`then_1`
          (bind _return_value (`self.CheckForBoundry` (`self.secondWheelIndex`) 10))
          (bind _output_get (set `self.secondWheelIndex` _return_value)))
        (:`then_2`
          (goto _label))
        (:`then_3`
          (goto _label_2))))))

(event `InputAction|Interact`
  (params (Key :type "Key Structure" :default "AnyKey"))
  (:`Pressed`
    (if (and (== (`.HitComponent` (`GameplayStatics.BreakHitResult` (`PlayerController.GetHitResultUnderCursorByChannel` (`GameplayStatics.GetPlayerController` 0) "TraceTypeQuery1" false))) (`self.thirdNumWheel`)) (`self.isLocked_0`))
      (`|ExecutionSequence`
        (:`then_1`
          (bind _return_value (`self.CheckForBoundry` (`self.thirdWheelIndex`) 10))
          (bind _output_get (set `self.thirdWheelIndex` _return_value)))
        (:`then_2`
          (goto _label))
        (:`then_3`
          (goto _label_2))))))

(fn `CheckForBoundry`
  (params (Value :type Integer) (Boundry :type Integer))
  (returns (`Return Value` :type Integer))
  (bind _result (`/Engine/EditorBlueprintResources/StandardMacros.IncrementInt` Value)
    (:`  `
      (if (>= Value Boundry)
        (return 0)
        (else
          (return _result))))))

(fn `DisableLock`
  (`|ExecutionSequence`
    (:`then_0`
      (`SceneComponent.SetVisibility` (`self.lockMesh`) false false))
    (:`then_1`
      (`SceneComponent.SetVisibility` (`self.firstNumWheel`) false false))
    (:`then_2`
      (`SceneComponent.SetVisibility` (`self.secondNumWheel`) false false))
    (:`then_3`
      (`SceneComponent.SetVisibility` (`self.thirdNumWheel`) false false))))

(fn `PlayUnlockSound`
  (`AudioComponent.Play` (`self.unlockSound`) 0.0))

(fn `SetMeshRotation`
  (params (Component :type "StaticMeshComponent Object Reference") (RotationIndex :type Integer) (AngleToRotate :type "Float (double-precision)") (RotationSpeed :type "Float (double-precision)"))
  (bind _returnvalue (* RotationIndex AngleToRotate))
  (if (< (.roll (`SceneComponent.GetSocketRotation` Component "None")) (- _returnvalue 0.2))
    (`SceneComponent.K2_SetRelativeRotation` Component (`KismetMathLibrary.RInterpTo` (`SceneComponent.GetSocketRotation` Component "None") (`KismetMathLibrary.MakeRotator` _returnvalue 0.0) (`GameplayStatics.GetWorldDeltaSeconds`) RotationSpeed) false false)
    (else
      (`SceneComponent.K2_SetRelativeRotation` Component (`KismetMathLibrary.MakeRotator` _returnvalue) false false))))

(fn `UserConstructionScript`)