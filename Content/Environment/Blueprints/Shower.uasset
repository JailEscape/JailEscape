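; Interactable shower actor that plays a drop sound and raises an Activator flag when the player interacts with it.
; Overlapping InteractZone enables input for the first-person character, and leaving disables it unless a dialog is open.
; The Interact press requires InteractObject to be under the cursor in a visibility trace.
; Tick clears Activator every frame, making it a short pulse with no reader in this graph.
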(event `self.interactZone.OnComponentBeginOverlap`
  (params (OverlappedComponent :type "PrimitiveComponent Object Reference") (OtherActor :type "Actor Object Reference") (OtherComp :type "PrimitiveComponent Object Reference") (OtherBodyIndex :type Integer) (bFromSweep :type Boolean) (SweepResult :type "HitResult Structure (by ref)"))
  (cast `/Game/FirstPersonCPP/Blueprints/FirstPersonCharacter` OtherActor)
  (`self.EnableInput` (`GameplayStatics.GetPlayerController` 0))
  (`KismetSystemLibrary.PrintString` "Input Enabled" false false (struct :`G` 0.66 :`B` 1.0 :`A` 1.0) 4.0))

(event `self.interactZone.OnComponentEndOverlap`
  (params (OverlappedComponent :type "PrimitiveComponent Object Reference") (OtherActor :type "Actor Object Reference") (OtherComp :type "PrimitiveComponent Object Reference") (OtherBodyIndex :type Integer))
  (bind _asfirst_person_character (cast `/Game/FirstPersonCPP/Blueprints/FirstPersonCharacter` OtherActor))
  (if (not (`MyProjectCharacter.isDialogOpen` _asfirst_person_character))
    (`self.DisableInput` (`GameplayStatics.GetPlayerController` 0))
    (`KismetSystemLibrary.PrintString` "Input Disabled" false false (struct :`G` 0.66 :`B` 1.0 :`A` 1.0) 4.0)))

(event `self.ReceiveTick`
  (params (DeltaSeconds :type "Float (single-precision)"))
  (set `self.activator` false))

(event `InputAction|Interact`
  (params (Key :type "Key Structure" :default "AnyKey"))
  (:`Pressed`
    (if (== (`.HitComponent` (`GameplayStatics.BreakHitResult` (`PlayerController.GetHitResultUnderCursorByChannel` (`GameplayStatics.GetPlayerController` 0) "TraceTypeQuery1" false))) (`self.interactObject`))
      (`|ExecutionSequence`
        (:`then_0`
          (`AudioComponent.Play` (`self.dropAudio`) 0.0))
        (:`then_1`
          (set `self.activator` true))))))

(fn `UserConstructionScript`)